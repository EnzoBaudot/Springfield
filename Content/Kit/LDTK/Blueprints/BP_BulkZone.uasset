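; BP_BulkZone is a level design kit volume that marks a labelled box or sphere zone in the editor and destroys itself on BeginPlay.
; Its construction script sets the text to the actor's display name, shows the selected shape and scales that shape's mesh to the component's extent or radius.
; A dynamic material instance applies colour and opacity, while per-shape 3D toggles control whether the solid mesh is visible.
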(event Custom|SetSphere
  ;[1 1 1] Set Sphere event
  (Rendering|SetVisibility (Variables|Default|GetBox) false false)
  (Rendering|SetVisibility (Variables|Default|GetSphere) true false)
  (Transformation|SetWorldScale3D (Variables|Default|GetSphereMesh) (Math|Conversions|ToVector(Float) (/ (Components|Sphere|GetScaledSphereRadius (Variables|Default|GetSphere)) 5e+01))))

(event Custom|3DCubeVis
  (bind _cubemesh (Variables|Default|GetCubeMesh))
  ;[1 1 1] 3D mesh visibility
  (if (Variables|Shape|Get3DCube)
    (Rendering|SetVisibility _cubemesh true false)
    (else
      (Rendering|SetVisibility _cubemesh false false))))

(event Custom|3DSphereVis
  (bind _spheremesh (Variables|Default|GetSphereMesh))
  ;[1 1 1] 3D mesh visibility
  (if (Variables|Shape|Get3DSphere)
    (Rendering|SetVisibility _spheremesh true false)
    (else
      (Rendering|SetVisibility _spheremesh false false))))

(event EventBeginPlay
  ;[0 1 0.03151] Destroy BP_Bulkzone on begin
  (Actor|DestroyActor))

(fn ConstructionScript
  (bind _sphere (Variables|Default|GetSphere))
  (bind _box (Variables|Default|GetBox))
  ;[1 1 1] Creates dynamic material instance and preps the meshes to be used
  (Rendering|Components|TextRender|SetText (Variables|Default|GetTextRender) (Utilities|Text|ToText(String) (Utilities|GetDisplayName self)))
  (bind _returnvalue (Rendering|Material|CreateDynamicMaterialInstance "/Game/Kit/LDTK/Materials/M_Sphere.M_Sphere" "" "None" :!class /Script/Engine.KismetMaterialLibrary))
  (LocalVariables|SetDynamMat _returnvalue)
  (Rendering|Material|SetMaterial (Variables|Default|GetSphereMesh) 0 (LocalVariables|GetDynamMat))
  (Rendering|Material|SetMaterial (Variables|Default|GetCubeMesh) 0 (LocalVariables|GetDynamMat))
  (Rendering|Material|SetScalarParameterValue (LocalVariables|GetDynamMat) "Opacity" (Variables|Shape|GetOpacity) :!class /Script/Engine.MaterialInstanceDynamic)
  (Rendering|Material|SetVectorParameterValue (LocalVariables|GetDynamMat) "Colour" (Variables|Shape|GetColour) :!class /Script/Engine.MaterialInstanceDynamic)
  (switch Utilities|FlowControl|Switch|SwitchonShape_Enum (Variables|Shape|GetShape)
    (:NewEnumerator0
      (Rendering|SetVisibility _sphere false false)
      (Rendering|SetVisibility _box true false)
      (Transformation|SetWorldScale3D (Variables|Default|GetCubeMesh) (/ (Components|Box|GetScaledBoxExtent (Variables|Default|GetBox)) 5e+01))
      (CallFunction|3DCubeVis))
    (:NewEnumerator1
      (Rendering|SetVisibility _box false false)
      (Rendering|SetVisibility _sphere true false)
      (Transformation|SetWorldScale3D (Variables|Default|GetSphereMesh) (Math|Conversions|ToVector(Float) (/ (Components|Sphere|GetScaledSphereRadius (Variables|Default|GetSphere)) 5e+01)))
      (CallFunction|3DSphereVis))))