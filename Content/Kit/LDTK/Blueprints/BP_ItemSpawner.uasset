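; BP_ItemSpawner spawns an Item actor at its Billboard on a repeating timer, using a fixed or random delay.
; Each ItemSpawner call re-sets the timer on itself, then spawns always or only when the last item is invalid or its transform differs from the Billboard's beyond set tolerances.
; A separate Preview event spawns the item once, without tracking it.
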(event Custom|Preview
  (bind _billboard (Variables|Default|GetBillboard))
  (bind _returnvalue (Transformation|GetWorldTransform _billboard))
  (Game|SpawnActorfromClass (Variables|Default|GetItem) (Math|Transform|MakeTransform (.location _returnvalue) (.rotation _returnvalue) (Variables|Default|GetScale)) "Undefined" 0 0))

(event Custom|ItemSpawner
  (bind _billboard (Variables|Default|GetBillboard))
  (bind _returnvalue (Transformation|GetWorldTransform _billboard))
  (Utilities|Time|SetTimerbyEvent (delegate Custom|ItemSpawner) (select (Variables|Default|GetRandomDelay) (Math|Random|RandomFloatinRange (Variables|Default|GetMinSpawnDelay) (Variables|Default|GetMaxSpawnDelay)) (Variables|Default|GetMinSpawnDelay)) true)
  (if (Variables|Default|GetAlwaysSpawn)
    (bind _returnvalue_2 (Game|SpawnActorfromClass (Variables|Default|GetItem) (Math|Transform|MakeTransform (.location _returnvalue) (.rotation _returnvalue) (Variables|Default|GetScale)) "Undefined" 0 0 :!label _label))
    (Variables|Default|SetSpawnedItem _returnvalue_2)
    (else
      (Utilities|IsValid (Variables|Default|GetSpawnedItem)
        (:Is%20Valid
          (if (not (Class|KismetMathLibrary|NearlyEqualTransformTransform (Transformation|GetActorTransform (Variables|Default|GetSpawnedItem)) (Transformation|GetWorldTransform (Variables|Default|GetBillboard)) 5e+01 5e+01 1.0))
            (goto _label)))
        (:Is%20Not%20Valid
          (goto _label))))))

(event EventBeginPlay
  (CallFunction|ItemSpawner))

(fn ConstructionScript)