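; RoomDescription is a demo room display stand that shows a title and a description as text.
; The construction script creates dynamic material instances on the base and flat wall meshes and sets their Color parameter from StandColor.
; It also applies the Title and Description strings and their world sizes to the two text components.
; The event graph has no active logic.
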(event EventBeginPlay)

(event EventActorBeginOverlap
  (params (OtherActor :type Actor%20Object%20Reference)))

(event EventTick
  (params (DeltaSeconds :type Float%20%28single-precision%29)))

(fn ConstructionScript
  (bind _returnvalue (Rendering|Material|CreateDynamicMaterialInstance (Variables|Default|GetSM_Base) 3 0 "None" :!class /Script/Engine.PrimitiveComponent))
  (Rendering|Material|SetVectorParameterValue _returnvalue "Color" (Variables|Default|GetStandColor) :!class /Script/Engine.MaterialInstanceDynamic)
  (bind _returnvalue_2 (Rendering|Material|CreateDynamicMaterialInstance (Variables|Default|GetSM_Base_FlatWall) 0 0 "None" :!class /Script/Engine.PrimitiveComponent))
  (Rendering|Material|SetVectorParameterValue _returnvalue_2 "Color" (Variables|Default|GetStandColor) :!class /Script/Engine.MaterialInstanceDynamic)
  (Rendering|Components|TextRender|SetText (Variables|Default|GetTitleText) (Variables|Default|GetTitle))
  (Rendering|Components|TextRender|SetText (Variables|Default|GetDescriptionText) (Variables|Default|GetDescription))
  (Rendering|Components|TextRender|SetWorldSize (Variables|Default|GetTitleText) (Variables|Default|GetTitleSize))
  (Rendering|Components|TextRender|SetWorldSize (Variables|Default|GetDescriptionText) (Variables|Default|GetDescriptionSize)))