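; BP_Kettle-01 is a configurable medieval kettle prop from the props kit, with no active runtime logic.
; Its construction script runs a chain of macros that toggle visibility and collision on optional mesh parts: handle, binding, cap and three sticks, each driven by a boolean.
; A final macro sets the handle mesh's relative X rotation from a HandleRotation variable.
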(event EventBeginPlay)

(event EventActorBeginOverlap
  (params (OtherActor :type Actor%20Object%20Reference)))

(event EventTick
  (params (DeltaSeconds :type Float%20%28single-precision%29)))

(fn ConstructionScript
  ;[1 1 1] Enable/disable. Macro (Visibility and Enable/Disable collision)
  (Utilities|Enabled/DisabledMacro (Variables|Default|GetHandle%20Enabled) (Variables|Default|GetStaticMeshComponent02)
    (:Resume
      (Utilities|Enabled/DisabledMacro (Variables|Default|GetBinding%20Enabled) (Variables|Default|GetStaticMeshComponent03)
        (:Resume
          (Utilities|Enabled/DisabledMacro (Variables|Default|GetCap%201%20Enabled) (Variables|Default|GetStaticMeshComponent05)
            (:Resume
              (Utilities|Enabled/DisabledMacro (Variables|Default|GetStick%201%20Enabled) (Variables|Default|GetStaticMeshComponent06)
                (:Resume
                  (Utilities|Enabled/DisabledMacro (Variables|Default|GetStick%202%20Enabled) (Variables|Default|GetStaticMeshComponent01)
                    (:Resume
                      (Utilities|Enabled/DisabledMacro (Variables|Default|GetStick%203%20Enabled) (Variables|Default|GetStaticMeshComponent0)
                        (:Resume
                          ;[1 1 1] Handle Rotation
                          (Utilities|RelativeRotationMacro (Variables|Default|GetStaticMeshComponent02) (Variables|Default|GetHandle%20Rotation) 0.0 0.0))))))))))))))